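; BP_Spawner is a spawner actor that gathers candidate spawn locations from its child components, with no spawning logic yet.
; On BeginPlay it loops over the direct children of DefaultSceneRoot and stores each one's relative, not world, location in SpawnLocations.
; Tick prints the array's length every frame as debug output.
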(event `self.ReceiveBeginPlay`
  (for _array_element (`SceneComponent.GetChildrenComponents` (`self.DefaultSceneRoot`) false)
    (`KismetArrayLibrary.Array_Add` (`self.SpawnLocations`) (`SceneComponent.RelativeLocation` _array_element))))

(event `self.ReceiveTick`
  (params (DeltaSeconds :type "Float (single-precision)"))
  (`KismetSystemLibrary.PrintString` (`KismetStringLibrary.Conv_IntToString` (`KismetArrayLibrary.Array_Length` (`self.SpawnLocations`)))))

(fn `UserConstructionScript`)